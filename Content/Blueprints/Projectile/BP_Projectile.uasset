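; BP_Projectile is a team-aware damaging projectile actor that destroys itself after a short lifetime.
; Shoot stores the direction and damage causer, launches ProjectileMovement horizontally at Power speed with vertical velocity zeroed, and enables query collision on the Sphere, disabled at BeginPlay.
; Sphere overlaps with a BP_Character on a different team from the causer call its OnApplyDamageEvent with the projectile's forward vector, without destroying the projectile.
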(event `self.ReceiveBeginPlay`
  (`PrimitiveComponent.SetCollisionEnabled` (`self.Sphere`) "NoCollision")
  (`KismetSystemLibrary.Delay` 3.0)
  (`self.K2_DestroyActor`))

(event `self.Sphere.OnComponentBeginOverlap`
  (params (OverlappedComponent :type "PrimitiveComponent Object Reference") (OtherActor :type "Actor Object Reference") (OtherComp :type "PrimitiveComponent Object Reference") (OtherBodyIndex :type Integer) (bFromSweep :type Boolean) (SweepResult :type "HitResult Structure (by ref)"))
  (bind _asbp_character (cast `/Game/Blueprints/Character/BP_Character` OtherActor))
  (if (`|EnumInequality` (`/Game/Blueprints/Character/BP_Character.Team` _asbp_character) (`/Game/Blueprints/Character/BP_Character.Team` (`self.DamageCauser`)))
    (`/Game/Blueprints/Character/BP_Character.OnApplyDamage_Event` _asbp_character 1.0 (`KismetMathLibrary.GetForwardVector` (`self.K2_GetActorRotation`)) (`self.DamageCauser`))))

(fn `Shoot`
  (params (ShootDirection :type "Vector Structure") (DamageCauser :type "/Game/Blueprints/Character/BP_Character Object Reference"))
  (bind (_returnvalue_x _returnvalue_y) (`KismetMathLibrary.BreakVector` (* (`self.Diretion`) (`self.Power`))))
  (set `self.Diretion` ShootDirection)
  (set `self.DamageCauser` DamageCauser)
  (set `MovementComponent.Velocity` (`KismetMathLibrary.MakeVector` _returnvalue_x _returnvalue_y) (`self.ProjectileMovement`))
  (`PrimitiveComponent.SetCollisionEnabled` (`self.Sphere`) "QueryOnly"))

(fn `UserConstructionScript`)