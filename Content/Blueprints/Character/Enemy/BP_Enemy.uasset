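; BP_Enemy is an enemy character that extends a parent character Blueprint and shuts down its AI on death.
; The construction script assigns its Team enum before running the parent's script.
; The Dead override calls StopAI, then the parent's Dead.
; StopAI casts to BP_EnemyController, sets the IsStopAI blackboard flag and stops the brain component's logic.
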(fn `Dead`
  (`self.StopAI`)
  (`parent.Dead`))

(fn `StopAI`
  (bind _asbp_enemy_controller (cast `/Game/Blueprints/Character/Enemy/BP_EnemyController` (`self.GetController`)))
  (`BlackboardComponent.SetValueAsBool` (`AIController.Blackboard` _asbp_enemy_controller) "IsStopAI" true)
  (`BrainComponent.StopLogic` (`AIController.BrainComponent` (`AIBlueprintHelperLibrary.GetAIController` _asbp_enemy_controller)) "Dead"))

(fn `UserConstructionScript`
  (set `self.Team` "NewEnumerator1")
  (`parent.UserConstructionScript`))