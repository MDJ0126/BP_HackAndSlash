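; Siege minion enemy character that fires projectiles from its front muzzle.
; The construction script sets its data name and fire and hit-react montages, assigns Projectile from a world lookup of an existing projectile actor, then runs the parent script.
; FireProjectile ignores that reference, spawning a new projectile at the Muzzle_Front socket and shooting it along the actor's forward vector with itself as damage causer.
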(fn `FireProjectile`
  (bind _returnvalue (`|SpawnActorFromClass` "/Game/Blueprints/Character/Enemy/Minion_Siege/BP_Minion_Siege_Projectile.BP_Minion_Siege_Projectile_C" (`KismetMathLibrary.Conv_VectorToTransform` (`SceneComponent.GetSocketLocation` (`self.Mesh`) "Muzzle_Front")) "Undefined" "MultiplyWithRoot" null null))
  (`/Game/Blueprints/Projectile/BP_Projectile.Shoot` _returnvalue (`KismetMathLibrary.GetForwardVector` (`self.K2_GetActorRotation`)) self))

(fn `UserConstructionScript`
  (set `self.CharacterDataName` "Minion_siege")
  (set `self.AttackAnim` "/Game/Blueprints/Character/Enemy/Minion_Siege/AM_Minion_Siege_Fire.AM_Minion_Siege_Fire")
  (set `self.HitAnim` "/Game/Blueprints/Character/Enemy/Minion_Siege/AM_HitReact.AM_HitReact")
  (bind _returnvalue (`GameplayStatics.GetActorOfClass` "/Game/Blueprints/Character/Enemy/Minion_Siege/BP_Minion_Siege_Projectile.BP_Minion_Siege_Projectile_C"))
  (set `self.Projectile` _returnvalue)
  (`parent.UserConstructionScript`))