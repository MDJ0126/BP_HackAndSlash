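; Base playable character that maps Enhanced Input to camera-relative movement, a cursor-aimed montage combo attack and cooldown-gated special and ultimate skills.
; SpecialAttack and Ultimate are stubs returning false, receiving input phases from wrappers that apply cooldowns on success.
; BeginPlay fills HUD skill slots and binds OnDamaged to raise ComboStack with a brief global slow-motion hit-stop.
; Guide meshes preview skill areas; knockback, ragdoll and destroy overrides suppress parent behavior.
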(event `self.ReceiveBeginPlay`
  (`parent.ReceiveBeginPlay`)
  (`self.HideSkillGuide`)
  (bind _asbp_player_controller (cast `/Game/Blueprints/Character/PlayerbleCharacter/BP_PlayerController` (`self.GetController`)))
  (set `self.PlayerController` _asbp_player_controller)
  (add `self.OnDamaged` (delegate `CustomEvent`))
  (`|ExecutionSequence`
    (:`then_0`
      (bind _aswbp_widget_name_tag (cast `/Game/Blueprints/UI/WBP_Widget_NameTag` (`WidgetComponent.GetUserWidgetObject` (`self.Widget NameTag`))))
      (`/Game/Blueprints/UI/WBP_Widget_NameTag.SetNameTag` _aswbp_widget_name_tag ""))
    (:`then_1`
      (bind _aswbp_widget_hp_bar (cast `/Game/Blueprints/UI/WBP_Widget_HpBar` (`WidgetComponent.GetUserWidgetObject` (`self.Widget HpBar`))))
      (`Widget.SetVisibility` _aswbp_widget_hp_bar "Hidden"))
    (:`then_2`
      (bind _asbp_player_controller_2 (cast `/Game/Blueprints/Character/PlayerbleCharacter/BP_PlayerController` (`self.GetController`)))
      (`|ExecutionSequence`
        (:`then_0`
          (bind _gameui (`/Game/Blueprints/Character/PlayerbleCharacter/BP_PlayerController.GameUI` _asbp_player_controller_2))
          (`/Game/Blueprints/UI/WBP_GameUI.SetSkillSlot1` _gameui (`self.SkillInfo1`)))
        (:`then_1`
          (`/Game/Blueprints/UI/WBP_GameUI.SetSkillSlot2` _gameui (`self.SkillInfo2`)))
        (:`then_2`
          (`/Game/Blueprints/UI/WBP_GameUI.SetSkillSlot3` _gameui (`self.SkillInfo3`)))))))

(event `CustomEvent`
  (bind _result (`/Engine/EditorBlueprintResources/StandardMacros.IncrementInt` (`self.ComboStack`))
    (:`  `
      (`self.OnUpdateComboStack` _result)
      (`GameplayStatics.SetGlobalTimeDilation` 0.2)
      (`KismetSystemLibrary.Delay` 0.03)
      (`GameplayStatics.SetGlobalTimeDilation` 1.0))))

(event `EnhancedInput|/Game/Blueprints/Input/IA_Look`
  (params (ActionValue :type "Vector2D Structure") (ElapsedSeconds :type "Float (double-precision)") (TriggeredSeconds :type "Float (double-precision)") (InputAction :type "InputAction Object Reference" :default "/Game/Blueprints/Input/IA_Look.IA_Look"))
  ; Look
)

(event `EnhancedInput|/Game/Blueprints/Input/IA_Move`
  (params (ActionValue :type "Vector2D Structure") (ElapsedSeconds :type "Float (double-precision)") (TriggeredSeconds :type "Float (double-precision)") (InputAction :type "InputAction Object Reference" :default "/Game/Blueprints/Input/IA_Move.IA_Move"))
  ; Movement
  (:`Triggered`
    (`self.UpdateMovement` ActionValue_X ActionValue_Y)))

(event `EnhancedInput|/Game/Blueprints/Input/IA_Attack1`
  (params (ActionValue :type Boolean) (ElapsedSeconds :type "Float (double-precision)") (TriggeredSeconds :type "Float (double-precision)") (InputAction :type "InputAction Object Reference" :default "/Game/Blueprints/Input/IA_Attack1.IA_Attack1"))
  ; Normal Attack
  (:`Triggered`
    (if (`self.IsCanUseInput`)
      (`self.NormalAttack`)
      (bind (_result _direction) (`self.GetForwardDirectionByCursor`))
      (if _result
        (`self.ShowSkillGuideCircle` (`self.K2_GetActorLocation`) _direction 140.0 3.0))))
  (:`Completed`
    (`self.HideSkillGuide`)))

(event `EnhancedInput|/Game/Blueprints/Input/IA_Attack2`
  (params (ActionValue :type Boolean) (ElapsedSeconds :type "Float (double-precision)") (TriggeredSeconds :type "Float (double-precision)") (InputAction :type "InputAction Object Reference" :default "/Game/Blueprints/Input/IA_Attack2.IA_Attack2"))
  ; Special Attack
  (:`Triggered`
    (`self.SpecialAttackProcess` "NewEnumerator1"))
  (:`Started`
    (`self.SpecialAttackProcess` "NewEnumerator0"))
  (:`Completed`
    (`self.SpecialAttackProcess` "NewEnumerator2")))

(event `EnhancedInput|/Game/Blueprints/Input/IA_Ultimate`
  (params (ActionValue :type Boolean) (ElapsedSeconds :type "Float (double-precision)") (TriggeredSeconds :type "Float (double-precision)") (InputAction :type "InputAction Object Reference" :default "/Game/Blueprints/Input/IA_Ultimate.IA_Ultimate"))
  ; Ultimate (R)
  (:`Triggered`
    (`self.UltimateProcess` "NewEnumerator1"))
  (:`Started`
    (`self.UltimateProcess` "NewEnumerator0"))
  (:`Completed`
    (`self.UltimateProcess` "NewEnumerator2")))

(fn `ApplyRagdoll`)

(fn `Damaged`
  (params (Damage :type "Float (double-precision)") (ShotFromDirection :type "Vector Structure") (DamageCauser :type "/Game/Blueprints/Character/BP_Character Object Reference"))
  (returns (IsDead :type Boolean))
  (bind _isdead (`parent.Damaged` Damage ShotFromDirection DamageCauser))
  (set `self.ComboCount` 0)
  (return _isdead))

(fn `DestroyActor`)

(fn `EndAttack`
  (bind _charactermovement (`self.CharacterMovement`))
  (set `self.bAttacking` false)
  (set `self.bCanNextAttack` false)
  (set `self.ComboCount` 0)
  (set `CharacterMovementComponent.bOrientRotationToMovement` true _charactermovement)
  (set `CharacterMovementComponent.MaxAcceleration` (`self.WalkMaxSpeed`) _charactermovement)
  (set `self.IsCanUseInput` true))

(fn `GetForwardDirectionByCursor`
  (returns (Result :type Boolean) (Direction :type "Vector Structure"))
  (locals (DirectionVector :type "Vector Structure"))
  (bind _playercontroller (`self.PlayerController`))
  (`/Engine/EditorBlueprintResources/StandardMacros.IsValid` _playercontroller
    (:`Is Valid`
      (bind (_result _location) (`/Game/Blueprints/Character/PlayerbleCharacter/BP_PlayerController.GetLocationUnderCursor` _playercontroller))
      (if _result
        (bind (_returnvalue_x _returnvalue_y) (`KismetMathLibrary.BreakVector` (- _location (`self.K2_GetActorLocation`))))
        (set `local.DirectionVector` (`KismetMathLibrary.Normal` (`KismetMathLibrary.MakeVector` _returnvalue_x _returnvalue_y)))
        (return true (`local.DirectionVector`))
        (else
          (return false (0.0 0.0 0.0)))))))

(fn `HideSkillGuide`
  (`SceneComponent.SetVisibility` (`self.SkillGuideSquare`) false false)
  (`SceneComponent.SetVisibility` (`self.SkillGuideCircle`) false false))

(fn `Knockback`
  (params (HitLocation :type "Vector Structure") (`Strength ` :type "Float (double-precision)"))
  ; 플레이어는 넉백 처리 안함
)

(fn `NormalAttack`
  (returns (SkillUsed :type Boolean))
  (`self.StartAttack`)
  (if (or (`self.bCanNextAttack`) (`AnimInstance.Montage_GetIsStopped` (`SkeletalMeshComponent.GetAnimInstance` (`self.Mesh`)) (`self.AttackAnim`)))
    (set `self.bAttacking` true)
    (if (== (`self.ComboCount`) 0)
      (`/Engine/EditorBlueprintResources/StandardMacros.IncrementInt` (`self.ComboCount`) :!label _label
        (:`  `
          (`self.PlayAnimMontage` (`self.AttackAnim`) 1.0 (`KismetSystemLibrary.MakeLiteralName` (`KismetStringLibrary.Conv_StringToName` (`KismetTextLibrary.Conv_TextToString` (`|FormatText` "Attack{0}" (`self.ComboCount`))))))
          (if (not (< (`self.ComboCount`) (`AnimMontage.GetNumSections` (`self.AttackAnim`))))
            (set `self.ComboCount` 0)
            (return true))))
      (elif (`self.bCanNextAttack`)
        (if (< (`self.ComboCount`) (`AnimMontage.GetNumSections` (`self.AttackAnim`)))
          (goto _label))))))

(fn `ShowSkillGuideCircle`
  (params (StartPosition :type "Vector Structure") (Direction :type "Vector Structure") (Radius :type "Float (double-precision)" :default 360.0) (Scale :type "Float (double-precision)" :default 1.0))
  (bind (_returnvalue_x _returnvalue_y _returnvalue_z) (`KismetMathLibrary.BreakVector` (* Scale (1.0 1.0 1.0))))
  (bind (_returnvalue_x_2 _returnvalue_y_2 _returnvalue_z_2) (`KismetMathLibrary.BreakVector` (`SceneComponent.K2_GetComponentLocation` (`self.SkillGuideCircleAxis`))))
  (bind _asbp_skill_guide_circle (cast `/Game/Blueprints/SkillGuide/BP_SkillGuideCircle` (`ChildActorComponent.ChildActor` (`self.SkillGuideCircle`))))
  (`/Game/Blueprints/SkillGuide/BP_SkillGuideCircle.SetGuideAngle` _asbp_skill_guide_circle Radius)
  (`SceneComponent.SetVisibility` (`self.SkillGuideCircle`) true false)
  (`SceneComponent.K2_SetWorldRotation` (`self.SkillGuideCircleAxis`) (`KismetMathLibrary.Conv_VectorToRotator` Direction) false false)
  (`SceneComponent.SetWorldScale3D` (`self.SkillGuideCircle`) (`KismetMathLibrary.MakeVector` 1.0 _returnvalue_y _returnvalue_z))
  (`SceneComponent.K2_SetWorldLocation` (`self.SkillGuideCircleAxis`) (`KismetMathLibrary.MakeVector` (.x StartPosition) (.y StartPosition) _returnvalue_z_2) false false))

(fn `ShowSkillGuideForwardSquare`
  (params (Direction :type "Vector Structure") (Width :type "Float (double-precision)" :default 1.0) (Height :type "Float (double-precision)" :default 1.0))
  (`SceneComponent.SetVisibility` (`self.SkillGuideSquare`) true false)
  (`SceneComponent.K2_SetWorldRotation` (`self.SkillGuideSquareAxis`) (`KismetMathLibrary.Conv_VectorToRotator` Direction) false false)
  (`SceneComponent.SetWorldScale3D` (`self.SkillGuideSquare`) (`KismetMathLibrary.MakeVector` 1.0 Width Height))
  (`SceneComponent.K2_SetRelativeLocation` (`self.SkillGuideSquare`) (`KismetMathLibrary.MakeVector` (* Height 100.0)) false false))

(fn `SpecialAttack`
  (params (InputPhase :type "/Game/Blueprints/Struct/EInputPhase Enum" :default "NewEnumerator0"))
  (returns (IsApplyCooltime :type Boolean))
  (return false))

(fn `SpecialAttackProcess`
  (params (InputPhase :type "/Game/Blueprints/Struct/EInputPhase Enum" :default "NewEnumerator0"))
  (bind _skillinfo2 (`self.SkillInfo2`))
  (if (`self.IsCanUseInput`)
    (bind _iscanuse (`self.CanUseSkill` (`self.SkillInfo2`)))
    (if _iscanuse
      (bind _isapplycooltime (`self.SpecialAttack` InputPhase))
      (if _isapplycooltime
        (`self.ApplyCooltimeSkill` (`self.SkillInfo2`))
        (set `self.ComboCount` 0))
      (elif (== InputPhase 0)
        (`/Game/Blueprints/Character/Variable/USkillInfo.OnUseSkill` _skillinfo2 _skillinfo2 false)))))

(fn `StartAttack`
  (bind _charactermovement (`self.CharacterMovement`))
  (if (not (`self.IsDead`))
    (set `CharacterMovementComponent.bOrientRotationToMovement` false _charactermovement)
    (set `CharacterMovementComponent.MaxAcceleration` (`self.CombatMaxSpeed`) _charactermovement)
    (bind (_result _direction) (`self.GetForwardDirectionByCursor`))
    (`self.K2_SetActorRotation` (`KismetMathLibrary.FindLookAtRotation` (`self.K2_GetActorLocation`) (+ _direction (`self.K2_GetActorLocation`))))))

(fn `Ultimate`
  (params (InputPhase :type "/Game/Blueprints/Struct/EInputPhase Enum" :default "NewEnumerator0"))
  (returns (IsApplyCooltime :type Boolean))
  (return false))

(fn `UltimateProcess`
  (params (InputPhase :type "/Game/Blueprints/Struct/EInputPhase Enum" :default "NewEnumerator0"))
  (bind _skillinfo3 (`self.SkillInfo3`))
  (if (`self.IsCanUseInput`)
    (bind _iscanuse (`self.CanUseSkill` (`self.SkillInfo3`)))
    (if _iscanuse
      (bind _isapplycooltime (`self.Ultimate` InputPhase))
      (if _isapplycooltime
        (`self.ApplyCooltimeSkill` (`self.SkillInfo3`))
        (set `self.ComboCount` 0))
      (elif (== InputPhase 0)
        (`/Game/Blueprints/Character/Variable/USkillInfo.OnUseSkill` _skillinfo3 _skillinfo3 false)))))

(fn `UpdateMovement`
  (params (X :type "Float (double-precision)") (Y :type "Float (double-precision)"))
  (bind (_returnvalue_roll _returnvalue_pitch _returnvalue_yaw) (`KismetMathLibrary.BreakRotator` (`SceneComponent.K2_GetComponentRotation` (`self.Camera`))))
  (bind (_returnvalue_roll_2 _returnvalue_pitch_2 _returnvalue_yaw_2) (`KismetMathLibrary.BreakRotator` (`SceneComponent.K2_GetComponentRotation` (`self.Camera`))))
  (bind _returnvalue (`KismetMathLibrary.Normal` (+ (* (`KismetMathLibrary.GetForwardVector` (`KismetMathLibrary.MakeRotator` 0.0 0.0 _returnvalue_yaw_2)) Y) (* (`KismetMathLibrary.GetRightVector` (`KismetMathLibrary.MakeRotator` 0.0 0.0 _returnvalue_yaw)) X))))
  (if (`self.IsCanUseInput`)
    (if (not (`self.IsDead`))
      (set `MovementComponent.Velocity` (* _returnvalue (`CharacterMovementComponent.MaxWalkSpeed` (`self.CharacterMovement`))) (`self.CharacterMovement`))
      (`self.K2_SetActorRotation` (`KismetMathLibrary.RInterpTo` (`self.K2_GetActorRotation`) (`KismetMathLibrary.MakeRotFromX` _returnvalue) (`GameplayStatics.GetWorldDeltaSeconds`) 5.0)))))

(fn `UserConstructionScript`
  (set `self.CharacterDataName` "Player")
  (set `self.Team` "NewEnumerator0")
  (set `self.HitAnim` "/Game/Blueprints/Character/PlayerbleCharacter/Kwang/AM_HitReact.AM_HitReact")
  (`parent.UserConstructionScript`))