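; Player controller that creates the game HUD, registers default Enhanced Input on possession and handles global keys.
; On BeginPlay it caches the game instance, finds the BP_Player actor and binds its HP and combo-stack dispatchers to update the HP bar and combo text in WBP_GameUI.
; The 1 key toggles the game instance's debug mode and Escape quits.
; A helper function returns the Visibility-trace hit location under the cursor.
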(event `self.ReceiveBeginPlay`
  (bind _asbp_game_instance (cast `/Game/Blueprints/Management/BP_GameInstance` (`GameplayStatics.GetGameInstance`)))
  (set `self.GameInstance` _asbp_game_instance)
  (bind _returnvalue (`GameplayStatics.GetActorOfClass` "/Game/Blueprints/Character/PlayerbleCharacter/BP_Player.BP_Player_C"))
  (bind _output_get (set `self.PlayerCharacter` _returnvalue))
  (add `/Game/Blueprints/Character/BP_Character.OnChangedHp` _output_get (delegate `OnChangedHp_이벤트`))
  (add `/Game/Blueprints/Character/PlayerbleCharacter/BP_Player.OnUpdateComboStack` (`self.PlayerCharacter`) (delegate `OnUpdateComboStack_이벤트`))
  (bind _returnvalue_2 (`|CreateWidget` "/Game/Blueprints/UI/WBP_GameUI.WBP_GameUI_C"))
  (set `self.GameUI` _returnvalue_2)
  (`UserWidget.AddToViewport` _returnvalue_2 0)
  (`/Game/Blueprints/UI/WBP_HpBar.UpdateHp` (`/Game/Blueprints/UI/WBP_GameUI.WBP_HpBar` _returnvalue_2) 1.0 1.0)
  (`/Game/Blueprints/UI/WBP_ComboText.SetComboStack` (`/Game/Blueprints/UI/WBP_GameUI.WBP_ComboText` _returnvalue_2) 0))

(event `OnChangedHp_이벤트`
  (params (CurrentHp :type "Float (double-precision)") (MaxHp :type "Float (double-precision)"))
  (`/Game/Blueprints/UI/WBP_HpBar.UpdateHp` (`/Game/Blueprints/UI/WBP_GameUI.WBP_HpBar` (`self.GameUI`)) CurrentHp MaxHp))

(event `OnUpdateComboStack_이벤트`
  (params (ComboStack :type Integer))
  (`/Game/Blueprints/UI/WBP_ComboText.SetComboStack` (`/Game/Blueprints/UI/WBP_GameUI.WBP_ComboText` (`self.GameUI`)) ComboStack))

(event `self.ReceivePossess`
  (params (PossessedPawn :type "Pawn Object Reference"))
  (if (`self.IsLocalPlayerController`)
    (`EnhancedInputSubsystemInterface.AddMappingContext` (pcsubsystem `EnhancedInputLocalPlayerSubsystem` self) "/Game/Blueprints/Input/IMC_Default.IMC_Default" 0 (struct))))

(event `Key|One`
  (params (Key :type "Key Structure"))
  (bind _gameinstance (`self.GameInstance`))
  (:`Pressed`
    (if (`/Game/Blueprints/Management/BP_GameInstance.IsDebugMode` (`self.GameInstance`))
      (set `/Game/Blueprints/Management/BP_GameInstance.IsDebugMode` false _gameinstance)
      (else
        (set `/Game/Blueprints/Management/BP_GameInstance.IsDebugMode` true _gameinstance)))))

(event `Key|Escape`
  (params (Key :type "Key Structure"))
  (:`Released`
    (`KismetSystemLibrary.QuitGame` null "Quit")))

(fn `GetLocationUnderCursor`
  (returns (Result :type Boolean) (Location :type "Vector Structure"))
  (bind (_hitresult _returnvalue) (`self.GetHitResultUnderCursorByChannel` "TraceTypeQuery1"))
  (return _returnvalue (`.Location` (`GameplayStatics.BreakHitResult` _hitresult))))

(fn `UserConstructionScript`)