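; BP_Character is a team-based combat character with data table stats, HP bar, name tag and three skill cooldown timers.
; Box and sphere traces damage other teams through an ApplyDamage dispatcher, feeding HP loss, knockback and hit feedback (montage, blood, overlay flash, camera shake).
; Super armor skips knockback and hit animation.
; Zero HP or falling triggers ragdoll death, decrements the GameMode spawn count and destroys the actor after a delay.
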(event `self.ReceiveBeginPlay`
  (add `self.OnApplyDamage` (delegate `OnApplyDamage_Event`))
  (`self.SetNameTag` (`self.Name`))
  (`self.UpdateHpBar`))

(event `OnApplyDamage_Event` :!signature `self.OnApplyDamage`
  (params (Damage :type "Float (double-precision)") (ShotFromDirection :type "Vector Structure") (DamageCauser :type "/Game/Blueprints/Character/BP_Character Object Reference"))
  (`self.DamagedProcess` Damage ShotFromDirection DamageCauser))

(event `self.ReceiveTick`
  (params (DeltaSeconds :type "Float (single-precision)"))
  (bind (_returnvalue_x _returnvalue_y _returnvalue_z) (`KismetMathLibrary.BreakVector` (`self.K2_GetActorLocation`)))
  (`|ExecutionSequence`
    (:`then_0`
      (`self.TickSkill` (`self.SkillInfo1`) DeltaSeconds))
    (:`then_1`
      (`self.TickSkill` (`self.SkillInfo2`) DeltaSeconds))
    (:`then_2`
      (`self.TickSkill` (`self.SkillInfo3`) DeltaSeconds))
    (:`then_3`
      ; 낙사 체크
      (if (< _returnvalue_z -100.0)
        (`self.DeadProcess`)))))

(fn `ApplyCooltimeSkill`
  (params (SkillInfo :type "/Game/Blueprints/Character/Variable/USkillInfo Object Reference"))
  (`/Game/Blueprints/Character/Variable/USkillInfo.UseSkill` SkillInfo))

(fn `ApplyRagdoll`
  (bind (_returnvalue_x _returnvalue_y) (`KismetMathLibrary.BreakVector` (`KismetMathLibrary.GetForwardVector` (`self.K2_GetActorRotation`))))
  ; Regdoll 처리 (https://wecandev.tistory.com/65)
  (`PrimitiveComponent.SetCollisionProfileName` (`self.Mesh`) "Ragdoll" true)
  (`PrimitiveComponent.SetCollisionEnabled` (`self.Mesh`) "QueryAndPhysics")
  (`PrimitiveComponent.SetSimulatePhysics` (`self.Mesh`) true)
  (`SkeletalMeshComponent.AddImpulseToAllBodiesBelow` (`self.Mesh`) (* (`KismetMathLibrary.MakeVector` _returnvalue_x _returnvalue_y -1.0) -400.0) "pelvis" true true))

(fn `CanUseSkill`
  (params (SkillInfo :type "/Game/Blueprints/Character/Variable/USkillInfo Object Reference"))
  (returns (IsCanUse :type Boolean))
  (bind _returnvalue (<= (`/Game/Blueprints/Character/Variable/USkillInfo.CoolTime` SkillInfo) 0.0))
  (if _returnvalue
    (return _returnvalue)))

(fn `Damaged`
  (params (Damage :type "Float (double-precision)") (ShotFromDirection :type "Vector Structure") (DamageCauser :type "/Game/Blueprints/Character/BP_Character Object Reference"))
  (returns (IsDead :type Boolean))
  (set `self.CurHp` (- (`self.CurHp`) Damage))
  (`self.OnChangedHp` (`self.CurHp`) (`self.MaxHp`))
  (if (not (`self.IsSuperArmor`))
    (`self.OnDamaged` DamageCauser)
    (`self.UpdateHpBar`)
    (`self.Knockback` ShotFromDirection 500.0)
    (return (<= (`self.CurHp`) 0.0))))

(fn `Dead`
  (bind _capsulecomponent (`self.CapsuleComponent`))
  (bind _charactermovement (`self.CharacterMovement`))
  (set `self.IsDead` true)
  (`self.OnDead`)
  (`self.SetActorTickEnabled` false)
  (`PrimitiveComponent.SetCollisionEnabled` _capsulecomponent "NoCollision")
  (`PrimitiveComponent.SetCollisionResponseToChannel` _capsulecomponent "ECC_Pawn" "ECR_Ignore")
  (bind _asbp_game_mode (cast `/Game/Blueprints/Management/BP_GameMode` (`GameplayStatics.GetGameMode`)))
  (`/Engine/EditorBlueprintResources/StandardMacros.DecrementInt` (`/Game/Blueprints/Management/BP_GameMode.CurrentSpawnCount` _asbp_game_mode)
    (:`  `
      (`self.ApplyRagdoll`)
      (`MovementComponent.StopMovementImmediately` _charactermovement)
      (`CharacterMovementComponent.DisableMovement` _charactermovement)
      (`SceneComponent.SetVisibility` (`self.Widget HpBar`) false false)
      (`SceneComponent.SetVisibility` (`self.Widget NameTag`) false false))))

(fn `DestroyActor`
  (`self.K2_DestroyActor`))

(fn `DisableActor`
  (`self.SetActorHiddenInGame` true)
  (`self.SetActorTickEnabled` false)
  (`self.SetActorEnableCollision` false)
  (set `self.IsActive` false))

(fn `EnableActor`
  (`self.SetActorHiddenInGame` false)
  (`self.SetActorTickEnabled` true)
  (`self.SetActorEnableCollision` true)
  (set `self.IsActive` true))

(fn `FireProjectile`)

(fn `Knockback`
  (params (HitLocation :type "Vector Structure") (`Strength ` :type "Float (double-precision)"))
  (if (not (`self.IsDead`))
    (`MovementComponent.StopMovementImmediately` (`self.CharacterMovement`))
    (`self.LaunchCharacter` (* (`KismetMathLibrary.Normal` (`KismetMathLibrary.MakeVector` (.x HitLocation) (.y HitLocation))) `Strength `))))

(fn `SetNameTag`
  (params (Name :type String))
  (bind _aswbp_widget_name_tag (cast `/Game/Blueprints/UI/WBP_Widget_NameTag` (`WidgetComponent.GetUserWidgetObject` (`self.Widget NameTag`))))
  (`/Game/Blueprints/UI/WBP_Widget_NameTag.SetNameTag` _aswbp_widget_name_tag Name))

(fn `TakeDamageForwardBox`
  (locals (DrawDebugTrace :type "EDrawDebugTrace Enum"))
  (bind _attackhitrage (`self.AttackHitRage`))
  (bind _returnvalue (+ (`self.K2_GetActorLocation`) (* (`self.GetActorForwardVector`) 100.0)))
  (bind _asbp_game_instance (cast `/Game/Blueprints/Management/BP_GameInstance` (`GameplayStatics.GetGameInstance`)))
  (if (`/Game/Blueprints/Management/BP_GameInstance.IsDebugMode` _asbp_game_instance)
    (set `local.DrawDebugTrace` "ForDuration")
    (else
      (set `local.DrawDebugTrace` "None")))
  (bind (_outhits _returnvalue_2) (`KismetSystemLibrary.BoxTraceMultiForObjects` :`Start` _returnvalue :`End` _returnvalue :`HalfSize` (`KismetMathLibrary.MakeVector` (* _attackhitrage 0.5) _attackhitrage 100.0) :`Orientation` (`self.K2_GetActorRotation`) :`ObjectTypes` (`|MakeArray` "ObjectTypeQuery3" :!type "EObjectTypeQuery Enum") :`DrawDebugType` (`local.DrawDebugTrace`) :`DrawTime` 0.5))
  (if _returnvalue_2
    (for _array_element _outhits
      (bind _asbp_character (cast `/Game/Blueprints/Character/BP_Character` (`.HitActor` (`GameplayStatics.BreakHitResult` _array_element))))
      (if (`|EnumInequality` (`/Game/Blueprints/Character/BP_Character.Team` _asbp_character) (`self.Team`))
        (`self.OnApplyDamage` _asbp_character (`self.Damage`) (`KismetMathLibrary.GetForwardVector` (`self.K2_GetActorRotation`)) self)))))

(fn `TakeDamageSphere`
  (locals (DrawDebugTrace :type "EDrawDebugTrace Enum"))
  (bind _returnvalue (`self.K2_GetActorLocation`))
  (bind _asbp_game_instance (cast `/Game/Blueprints/Management/BP_GameInstance` (`GameplayStatics.GetGameInstance`)))
  (if (`/Game/Blueprints/Management/BP_GameInstance.IsDebugMode` _asbp_game_instance)
    (set `local.DrawDebugTrace` "ForDuration")
    (else
      (set `local.DrawDebugTrace` "None")))
  (bind (_outhits _returnvalue_2) (`KismetSystemLibrary.SphereTraceMultiForObjects` :`Start` _returnvalue :`End` _returnvalue :`Radius` 800.0 :`ObjectTypes` (`|MakeArray` "ObjectTypeQuery3" :!type "EObjectTypeQuery Enum") :`DrawDebugType` (`local.DrawDebugTrace`)))
  (if _returnvalue_2
    (for _array_element _outhits
      (bind _asbp_character (cast `/Game/Blueprints/Character/BP_Character` (`.HitActor` (`GameplayStatics.BreakHitResult` _array_element))))
      (if (`|EnumInequality` (`/Game/Blueprints/Character/BP_Character.Team` _asbp_character) (`self.Team`))
        (`self.OnApplyDamage` _asbp_character (`self.Damage`) (`KismetMathLibrary.GetForwardVector` (`self.K2_GetActorRotation`)) self)))))

(fn `TickSkill`
  (params (SkillInfo :type "/Game/Blueprints/Character/Variable/USkillInfo Object Reference") (DeltaSeconds :type "Float (double-precision)"))
  (`/Engine/EditorBlueprintResources/StandardMacros.IsValid` SkillInfo
    (:`Is Valid`
      (if true
        (set `/Game/Blueprints/Character/Variable/USkillInfo.CoolTime` (`KismetMathLibrary.FMax` (- (`/Game/Blueprints/Character/Variable/USkillInfo.CoolTime` SkillInfo) DeltaSeconds)) SkillInfo)))))

(fn `UpdateHpBar`
  (bind _aswbp_widget_hp_bar (cast `/Game/Blueprints/UI/WBP_Widget_HpBar` (`WidgetComponent.GetUserWidgetObject` (`self.Widget HpBar`))))
  (`/Game/Blueprints/UI/WBP_Widget_HpBar.UpdateHp` _aswbp_widget_hp_bar (`self.CurHp`) (`self.MaxHp`)))

(fn `UserConstructionScript`
  (bind _returnvalue (`GameplayStatics.GetActorOfClass` "/Game/Blueprints/Projectile/BP_Projectile.BP_Projectile_C"))
  (set `self.Projectile` _returnvalue)
  (`|ExecutionSequence`
    (:`then_0`
      (bind _returnvalue_2 (`|GetDataTableRow` "/Game/DataTable/DT_Character.DT_Character" (`self.CharacterDataName`))
        (:`then`
          (set `self.Name` (break `/Game/DataTable/FCharacterData` _returnvalue_2))
          (bind _output_get (set `self.MaxHp` (`.Hp_17_1F22F6E84236F54D3E574198A7261C00` (break `/Game/DataTable/FCharacterData` _returnvalue_2))))
          (set `self.CurHp` _output_get)
          (set `self.Damage` (`.Damage_16_7DD27B28470A6A1A6C30DE8F75DC5909` (break `/Game/DataTable/FCharacterData` _returnvalue_2)))
          (set `CharacterMovementComponent.MaxWalkSpeed` (`.Speed_13_D596F80C4EFF37A3EBA91AB5BF8BF4BD` (break `/Game/DataTable/FCharacterData` _returnvalue_2)) (`self.CharacterMovement`))
          (set `self.AttackRange` (`.AttackRange_14_7BAE1D284EFECD41DE104AAF822BBD0A` (break `/Game/DataTable/FCharacterData` _returnvalue_2)))
          (set `self.AttackHitRage` (`.AttackHitRage_20_2A12FE6F4A533367AC64EBB523ED963C` (break `/Game/DataTable/FCharacterData` _returnvalue_2))))))))